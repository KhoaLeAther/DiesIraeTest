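; An interactable pillar Blueprint that changes its appearance when its interaction is triggered.
; On OnInteractionTriggered it runs the parent handler, then swaps its static mesh to a cone and sets that component's relative scale to unit size.
; The interaction trigger comes from the parent class; BeginPlay, overlap and Tick are disabled stubs, and the construction script only calls the parent.
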(event EventBeginPlay
  (|CallParentFunction) ; This node is disabled and will not be called.\nDrag off pins to build functionality.
)

(event Collision|EventActorBeginOverlap
  (params (OtherActor :type Actor%20Object%20Reference))
  (|CallParentFunction OtherActor) ; This node is disabled and will not be called.\nDrag off pins to build functionality.
)

(event EventTick
  (params (DeltaSeconds :type Float%20%28single-precision%29))
  (|CallParentFunction DeltaSeconds) ; This node is disabled and will not be called.\nDrag off pins to build functionality.
)

(event EventOnInteractionTriggered
  (params (InteractActor :type Actor%20Object%20Reference))
  (bind _staticmesh (Variables|Default|GetStaticMesh))
  (|CallParentFunction InteractActor)
  (Components|StaticMesh|SetStaticMesh _staticmesh "/Engine/BasicShapes/Cone.Cone")
  (Transformation|SetRelativeScale3D _staticmesh "1.000000,1.000000,1.000000"))

(fn ConstructionScript
  (|CallParentFunction))